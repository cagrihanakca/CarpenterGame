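; Game mode for a carpentry game that runs a single-order loop of randomly generated product requests.
; After a short random delay from BeginPlay, GenerateOrder fills CurrentOrder with a random product type and paint color, marks it active and broadcasts OnOrderGenerated.
; CompleteOrder deactivates the order, broadcasts OnOrderCompleted and restarts the random timer for the next one.
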(event `self.ReceiveBeginPlay`
  (`KismetSystemLibrary.K2_SetTimer` null "GenerateOrder" (`KismetMathLibrary.RandomFloatInRange` 5.0 15.0)))

(fn `CompleteOrder`
  (bind _structout (setmembers `/Game/S_Order` :`StructRef` (`self.CurrentOrder`) :`IsActive` false))
  (set `self.CurrentOrder` _structout)
  (`self.OnOrderCompleted`)
  (`KismetSystemLibrary.K2_SetTimer` null "GenerateOrder" (`KismetMathLibrary.RandomFloatInRange` 5.0 15.0)))

(fn `GenerateOrder`
  (bind _output_get (set `self.CurrentOrder` (make `/Game/S_Order` (cast `/Game/E_ProductType` (`KismetMathLibrary.Conv_IntToByte` (`KismetMathLibrary.RandomIntegerInRange` 0 3))) (cast `/Game/E_PaintColor` (`KismetMathLibrary.Conv_IntToByte` (`KismetMathLibrary.RandomIntegerInRange` 0 3))) true)))
  (`self.OnOrderGenerated` _output_get))

(fn `UserConstructionScript`)