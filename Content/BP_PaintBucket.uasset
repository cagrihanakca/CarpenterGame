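; Paint bucket actor that holds one paint color and passes it to the paint workbench that owns it.
; InitColor stores the color and switches the cylinder's material to the matching red, green, blue or yellow one.
; TriggerPaint casts the parent actor to BP_PaintWorkbench and calls its Paint with the stored color, so it expects to be a child actor of that workbench.
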(fn `InitColor`
  (params (Color :type "/Game/E_PaintColor Enum" :default "NewEnumerator0"))
  (bind _cylinder (`self.Cylinder`))
  (bind _output_get (set `self.PaintColor` Color))
  (switch `/Game/E_PaintColor` _output_get
    (:`NewEnumerator0`
      (`PrimitiveComponent.SetMaterial` _cylinder 0 "/Game/M_Red.M_Red"))
    (:`NewEnumerator1`
      (`PrimitiveComponent.SetMaterial` _cylinder 0 "/Game/M_Green.M_Green"))
    (:`NewEnumerator2`
      (`PrimitiveComponent.SetMaterial` _cylinder 0 "/Game/M_Blue.M_Blue"))
    (:`NewEnumerator3`
      (`PrimitiveComponent.SetMaterial` _cylinder 0 "/Game/M_Yellow.M_Yellow"))))

(fn `TriggerPaint`
  (bind _asbp_paint_workbench (cast `/Game/BP_PaintWorkbench` (`self.GetParentActor`)))
  (`/Game/BP_PaintWorkbench.Paint` _asbp_paint_workbench (`self.PaintColor`)))

(fn `UserConstructionScript`)