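; A paint workbench actor that recolors the product placed on it, with red, green, blue and yellow paint buckets.
; On BeginPlay it initializes each child-actor bucket with its color.
; A box overlap tracks the current BP_Product and clears it when a product leaves.
; The Paint function sets that product's color and swaps its static mesh material to match.
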(event `self.ReceiveBeginPlay`
  (bind _asbp_paint_bucket (cast `/Game/BP_PaintBucket` (`ChildActorComponent.ChildActor` (`self.RedPaintBucket`))))
  (`/Game/BP_PaintBucket.InitColor` _asbp_paint_bucket "NewEnumerator0")
  (bind _asbp_paint_bucket_2 (cast `/Game/BP_PaintBucket` (`ChildActorComponent.ChildActor` (`self.GreenPaintBucket`))))
  (`/Game/BP_PaintBucket.InitColor` _asbp_paint_bucket_2 "NewEnumerator1")
  (bind _asbp_paint_bucket_3 (cast `/Game/BP_PaintBucket` (`ChildActorComponent.ChildActor` (`self.BluePaintBucket`))))
  (`/Game/BP_PaintBucket.InitColor` _asbp_paint_bucket_3 "NewEnumerator2")
  (bind _asbp_paint_bucket_4 (cast `/Game/BP_PaintBucket` (`ChildActorComponent.ChildActor` (`self.YellowPaintBucket`))))
  (`/Game/BP_PaintBucket.InitColor` _asbp_paint_bucket_4 "NewEnumerator3"))

(event `self.Box.OnComponentBeginOverlap`
  (params (OverlappedComponent :type "PrimitiveComponent Object Reference") (OtherActor :type "Actor Object Reference") (OtherComp :type "PrimitiveComponent Object Reference") (OtherBodyIndex :type Integer) (bFromSweep :type Boolean) (SweepResult :type "HitResult Structure (by ref)"))
  (bind _asbp_product (cast `/Game/BP_Product` OtherActor))
  (set `self.CurrentObject` _asbp_product))

(event `self.Box.OnComponentEndOverlap`
  (params (OverlappedComponent :type "PrimitiveComponent Object Reference") (OtherActor :type "Actor Object Reference") (OtherComp :type "PrimitiveComponent Object Reference") (OtherBodyIndex :type Integer))
  (cast `/Game/BP_Product` OtherActor)
  (set `self.CurrentObject` null))

(fn `Paint`
  (params (Color :type "/Game/E_PaintColor Enum" :default "NewEnumerator0"))
  (bind _currentobject (`self.CurrentObject`))
  (bind _staticmesh (`/Game/BP_Product.StaticMesh` (`self.CurrentObject`)))
  (`/Engine/EditorBlueprintResources/StandardMacros.IsValid` _currentobject
    (:`Is Valid`
      (bind _output_get (set `/Game/BP_Product.CurrentColor` Color _currentobject))
      (switch `/Game/E_PaintColor` _output_get
        (:`NewEnumerator0`
          (`PrimitiveComponent.SetMaterial` _staticmesh 0 "/Game/M_Red.M_Red"))
        (:`NewEnumerator1`
          (`PrimitiveComponent.SetMaterial` _staticmesh 0 "/Game/M_Green.M_Green"))
        (:`NewEnumerator2`
          (`PrimitiveComponent.SetMaterial` _staticmesh 0 "/Game/M_Blue.M_Blue"))
        (:`NewEnumerator3`
          (`PrimitiveComponent.SetMaterial` _staticmesh 0 "/Game/M_Yellow.M_Yellow"))))))

(fn `UserConstructionScript`)