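; BP_CarvingMachine is a machine that produces shaped products on request from its carving interface widget.
; On BeginPlay it binds to the widget's OnProduceRequest event, then spawns a BP_Product at SpawnPoint and sets its mesh from the requested type.
; A Box trigger shows the mouse cursor and switches to Game and UI input while the carpenter character is inside, restoring game-only input on exit.
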(event `self.ReceiveBeginPlay`
  (bind _aswbp_carving_interface (cast `/Game/WBP_CarvingInterface` (`WidgetComponent.GetWidget` (`self.Widget`))))
  (add `/Game/WBP_CarvingInterface.OnProduceRequest` _aswbp_carving_interface (delegate `OnProduceRequest_Event`)))

(event `OnProduceRequest_Event`
  (params (ProductType :type "/Game/E_ProductType Enum" :default "NewEnumerator0"))
  (`self.ProduceObject` ProductType))

(event `self.Box.OnComponentBeginOverlap`
  (params (OverlappedComponent :type "PrimitiveComponent Object Reference") (OtherActor :type "Actor Object Reference") (OtherComp :type "PrimitiveComponent Object Reference") (OtherBodyIndex :type Integer) (bFromSweep :type Boolean) (SweepResult :type "HitResult Structure (by ref)"))
  (bind _returnvalue (`GameplayStatics.GetPlayerController` 0))
  (cast `/Game/BP_CarpenterCharacter` OtherActor)
  (set `PlayerController.bShowMouseCursor` true _returnvalue)
  (`WidgetBlueprintLibrary.SetInputMode_GameAndUIEx` _returnvalue null))

(event `self.Box.OnComponentEndOverlap`
  (params (OverlappedComponent :type "PrimitiveComponent Object Reference") (OtherActor :type "Actor Object Reference") (OtherComp :type "PrimitiveComponent Object Reference") (OtherBodyIndex :type Integer))
  (bind _returnvalue (`GameplayStatics.GetPlayerController` 0))
  (cast `/Game/BP_CarpenterCharacter` OtherActor)
  (set `PlayerController.bShowMouseCursor` false _returnvalue)
  (`WidgetBlueprintLibrary.SetInputMode_GameOnly` _returnvalue))

(fn `ProduceObject`
  (params (`Product Type` :type "/Game/E_ProductType Enum" :default "NewEnumerator0"))
  (bind _returnvalue (`|SpawnActorFromClass` "/Game/BP_Product.BP_Product_C" (`SceneComponent.K2_GetComponentToWorld` (`self.SpawnPoint`)) "Undefined" "MultiplyWithRoot" null null))
  (`self.SetProductMesh` _returnvalue `Product Type`))

(fn `SetProductMesh`
  (params (Product :type "/Game/BP_Product Object Reference") (ProductType :type "/Game/E_ProductType Enum" :default "NewEnumerator0"))
  (bind _staticmesh (`/Game/BP_Product.StaticMesh` Product))
  (switch `/Game/E_ProductType` ProductType
    (:`NewEnumerator0`
      (`StaticMeshComponent.SetStaticMesh` _staticmesh "/Engine/BasicShapes/Cube.Cube"))
    (:`NewEnumerator1`
      (`StaticMeshComponent.SetStaticMesh` _staticmesh "/Engine/BasicShapes/Cylinder.Cylinder"))
    (:`NewEnumerator2`
      (`StaticMeshComponent.SetStaticMesh` _staticmesh "/Engine/BasicShapes/Sphere.Sphere"))
    (:`NewEnumerator3`
      (`StaticMeshComponent.SetStaticMesh` _staticmesh "/Engine/BasicShapes/Cone.Cone"))))

(fn `UserConstructionScript`)