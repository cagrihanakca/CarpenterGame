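; Multiplayer carving machine where players pick a product on a widget and have it spawned as a BP_Product.
; A box overlap records the locally controlled carpenter and toggles cursor and input mode.
; Widget events route through that character's server requests, and SelectedProduct's OnRep updates the highlight on clients.
; ProduceObject resets the selection, then spawns only if the spawn point holds no product and the type is valid.
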(event `self.ReceiveBeginPlay`
  ; Bind Widget Dispatchers
  (bind _aswbp_carving_interface (cast `/Game/Blueprints/UI/WBP_CarvingInterface` (`WidgetComponent.GetWidget` (`self.Widget`))))
  (add `/Game/Blueprints/UI/WBP_CarvingInterface.OnProduceRequest` _aswbp_carving_interface (delegate `OnProduceRequest_Event`))
  (add `/Game/Blueprints/UI/WBP_CarvingInterface.OnSelectionChanged` _aswbp_carving_interface (delegate `OnSelectionChanged_Evenet`)))

(event `OnProduceRequest_Event`
  ; Bind Widget Dispatchers
  (`/Game/Blueprints/Characters/BP_CarpenterCharacter.ServerRequestProduce` (`self.InteractingPlayer`) self (`self.SelectedProduct`)))

(event `OnSelectionChanged_Evenet`
  (params (ProductType :type "/Game/DataTypes/E_ProductType Enum" :default "NewEnumerator0"))
  ; Bind Widget Dispatchers
  (`/Game/Blueprints/Characters/BP_CarpenterCharacter.ServerRequestSelect` (`self.InteractingPlayer`) self ProductType))

(event `self.Box.OnComponentBeginOverlap`
  (params (OverlappedComponent :type "PrimitiveComponent Object Reference") (OtherActor :type "Actor Object Reference") (OtherComp :type "PrimitiveComponent Object Reference") (OtherBodyIndex :type Integer) (bFromSweep :type Boolean) (SweepResult :type "HitResult Structure (by ref)"))
  (bind _returnvalue (`GameplayStatics.GetPlayerController` 0))
  ; Player Enter - Set Interacting Player
  (bind _asbp_carpenter_character (cast `/Game/Blueprints/Characters/BP_CarpenterCharacter` OtherActor))
  (if (`Pawn.IsLocallyControlled` _asbp_carpenter_character)
    (set `self.InteractingPlayer` _asbp_carpenter_character)
    (set `PlayerController.bShowMouseCursor` true _returnvalue)
    (`WidgetBlueprintLibrary.SetInputMode_GameAndUIEx` _returnvalue null)))

(event `self.Box.OnComponentEndOverlap`
  (params (OverlappedComponent :type "PrimitiveComponent Object Reference") (OtherActor :type "Actor Object Reference") (OtherComp :type "PrimitiveComponent Object Reference") (OtherBodyIndex :type Integer))
  (bind _returnvalue (`GameplayStatics.GetPlayerController` 0))
  ; Player Exit - Clear Interacting Player
  (bind _asbp_carpenter_character (cast `/Game/Blueprints/Characters/BP_CarpenterCharacter` OtherActor))
  (if (`Pawn.IsLocallyControlled` _asbp_carpenter_character)
    (set `self.InteractingPlayer` null)
    (set `PlayerController.bShowMouseCursor` false _returnvalue)
    (`WidgetBlueprintLibrary.SetInputMode_GameOnly` _returnvalue)))

(fn `ApplySelection`
  ; Apply Selection Highlight
  (bind _aswbp_carving_interface (cast `/Game/Blueprints/UI/WBP_CarvingInterface` (`WidgetComponent.GetWidget` (`self.Widget`))))
  (`/Game/Blueprints/UI/WBP_CarvingInterface.HighlightSelection` _aswbp_carving_interface (`self.SelectedProduct`)))

(fn `IsSpawnPointClear`
  (returns (ReturnValue :type Boolean))
  ; Check Spawn Point
  (return (== (`KismetArrayLibrary.Array_Length` (`PrimitiveComponent.GetOverlappingActors` (`self.SpawPointCollision`) "/Game/Blueprints/Products/BP_Product.BP_Product_C")) 0)))

(fn `OnRep_SelectedProduct`
  ; OnRep - Apply Selection
  (`self.ApplySelection`))

(fn `ProduceObject`
  (params (`Product Type` :type "/Game/DataTypes/E_ProductType Enum" :default "NewEnumerator0"))
  ; Spawn Product
  (set `self.SelectedProduct` "NewEnumerator4")
  (if (`self.IsSpawnPointClear`)
    (if (`|EnumInequality` `Product Type` "NewEnumerator4")
      (bind _returnvalue (`|SpawnActorFromClass` "/Game/Blueprints/Products/BP_Product.BP_Product_C" (`SceneComponent.K2_GetComponentToWorld` (`self.SpawnPoint`)) "Undefined" "MultiplyWithRoot" null null))
      (set `/Game/Blueprints/Products/BP_Product.ProductType` `Product Type` _returnvalue)
      (`/Game/Blueprints/Products/BP_Product.SetProductMesh` _returnvalue))))

(fn `SetSelection`
  (params (ProductType :type "/Game/DataTypes/E_ProductType Enum" :default "NewEnumerator0"))
  ; Set Selected Product
  (set `self.SelectedProduct` ProductType)
  (`self.ApplySelection`))

(fn `UserConstructionScript`)