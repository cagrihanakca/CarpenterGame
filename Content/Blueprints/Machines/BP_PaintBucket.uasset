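; BP_PaintBucket is an interactable paint bucket that applies its color to a product at its parent paint workbench.
; InitColor stores the color and sets the matching red, green, blue or yellow material on the bucket's cylinder.
; CanInteract always allows interaction with a paint prompt, and TriggerPaint casts the parent actor to BP_PaintWorkbench and passes the stored color to its Paint function.
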(fn `CanInteract`
  (returns (ReturnValue :type Boolean) (InteractionInfo :type "/Game/DataTypes/S_InteractionInfo Structure"))
  (return true (make `/Game/DataTypes/S_InteractionInfo` "Press \"E\" to paint" "/Game/Input/IA_Interact.IA_Interact")))

(fn `InitColor`
  (params (Color :type "/Game/DataTypes/E_PaintColor Enum" :default "NewEnumerator0"))
  (bind _cylinder (`self.Cylinder`))
  ; Initialize Bucket Color
  (bind _output_get (set `self.PaintColor` Color))
  (switch `/Game/DataTypes/E_PaintColor` _output_get
    (:`NewEnumerator0`
      (`PrimitiveComponent.SetMaterial` _cylinder 0 "/Game/Materials/M_Red.M_Red"))
    (:`NewEnumerator1`
      (`PrimitiveComponent.SetMaterial` _cylinder 0 "/Game/Materials/M_Green.M_Green"))
    (:`NewEnumerator2`
      (`PrimitiveComponent.SetMaterial` _cylinder 0 "/Game/Materials/M_Blue.M_Blue"))
    (:`NewEnumerator3`
      (`PrimitiveComponent.SetMaterial` _cylinder 0 "/Game/Materials/M_Yellow.M_Yellow"))))

(fn `TriggerPaint`
  ; Apply Paint to Product
  (bind _asbp_paint_workbench (cast `/Game/Blueprints/Machines/BP_PaintWorkbench` (`self.GetParentActor`)))
  (`/Game/Blueprints/Machines/BP_PaintWorkbench.Paint` _asbp_paint_workbench (`self.PaintColor`)))

(fn `UserConstructionScript`)