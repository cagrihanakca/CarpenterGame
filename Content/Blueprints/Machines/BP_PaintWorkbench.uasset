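; BP_PaintWorkbench is a machine that applies a chosen color to a product placed on it.
; On BeginPlay it assigns a color to each of its red, green, blue and yellow paint bucket child actors.
; A box overlap tracks the current BP_Product, clearing it whenever any product leaves.
; The Paint function sets that product's color and refreshes its paint material if the reference is valid.
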(event `self.ReceiveBeginPlay`
  ; Initialize Piant Buckets
  (bind _asbp_paint_bucket (cast `/Game/Blueprints/Machines/BP_PaintBucket` (`ChildActorComponent.ChildActor` (`self.RedPaintBucket`))))
  (`/Game/Blueprints/Machines/BP_PaintBucket.InitColor` _asbp_paint_bucket "NewEnumerator0")
  (bind _asbp_paint_bucket_2 (cast `/Game/Blueprints/Machines/BP_PaintBucket` (`ChildActorComponent.ChildActor` (`self.GreenPaintBucket`))))
  (`/Game/Blueprints/Machines/BP_PaintBucket.InitColor` _asbp_paint_bucket_2 "NewEnumerator1")
  (bind _asbp_paint_bucket_3 (cast `/Game/Blueprints/Machines/BP_PaintBucket` (`ChildActorComponent.ChildActor` (`self.BluePaintBucket`))))
  (`/Game/Blueprints/Machines/BP_PaintBucket.InitColor` _asbp_paint_bucket_3 "NewEnumerator2")
  (bind _asbp_paint_bucket_4 (cast `/Game/Blueprints/Machines/BP_PaintBucket` (`ChildActorComponent.ChildActor` (`self.YellowPaintBucket`))))
  (`/Game/Blueprints/Machines/BP_PaintBucket.InitColor` _asbp_paint_bucket_4 "NewEnumerator3"))

(event `self.Box.OnComponentBeginOverlap`
  (params (OverlappedComponent :type "PrimitiveComponent Object Reference") (OtherActor :type "Actor Object Reference") (OtherComp :type "PrimitiveComponent Object Reference") (OtherBodyIndex :type Integer) (bFromSweep :type Boolean) (SweepResult :type "HitResult Structure (by ref)"))
  ; Detect Product in Paint Area
  (bind _asbp_product (cast `/Game/Blueprints/Products/BP_Product` OtherActor))
  (set `self.CurrentObject` _asbp_product))

(event `self.Box.OnComponentEndOverlap`
  (params (OverlappedComponent :type "PrimitiveComponent Object Reference") (OtherActor :type "Actor Object Reference") (OtherComp :type "PrimitiveComponent Object Reference") (OtherBodyIndex :type Integer))
  ; Clear Current Product
  (cast `/Game/Blueprints/Products/BP_Product` OtherActor)
  (set `self.CurrentObject` null))

(fn `Paint`
  (params (Color :type "/Game/DataTypes/E_PaintColor Enum" :default "NewEnumerator0"))
  (bind _currentobject (`self.CurrentObject`))
  ; Paint Product
  (`/Engine/EditorBlueprintResources/StandardMacros.IsValid` _currentobject
    (:`Is Valid`
      (set `/Game/Blueprints/Products/BP_Product.Color` Color _currentobject)
      (`/Game/Blueprints/Products/BP_Product.SetPaintMaterial` (`self.CurrentObject`)))))

(fn `UserConstructionScript`)