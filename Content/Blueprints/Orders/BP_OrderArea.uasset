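; BP_OrderArea is a delivery zone in a carpenter game that scores products entering its box against the current order.
; On overlap it stores the product and, if the game state's order is active, compares product type and paint color.
; A full match pays full price, a wrong color half and a wrong type nothing.
; After a short delay, ProcessDelivery calls CompleteOrder on the game mode and destroys the product.
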(event `self.Box.OnComponentBeginOverlap`
  (params (OverlappedComponent :type "PrimitiveComponent Object Reference") (OtherActor :type "Actor Object Reference") (OtherComp :type "PrimitiveComponent Object Reference") (OtherBodyIndex :type Integer) (bFromSweep :type Boolean) (SweepResult :type "HitResult Structure (by ref)"))
  (bind (_currentorder_producttype _currentorder_paintcolor _currentorder_price) (break `/Game/DataTypes/S_Order` (`self.CurrentOrder`)))
  (bind (_currentorder_producttype_2 _currentorder_paintcolor_2 _currentorder_price_2) (break `/Game/DataTypes/S_Order` (`self.CurrentOrder`)))
  ; Check Active Order & Product
  (bind _asbp_product (cast `/Game/Blueprints/Products/BP_Product` OtherActor))
  (set `self.CurrentProduct` _asbp_product)
  (bind _asbp_carpenter_game_state (cast `/Game/Blueprints/BP_CarpenterGameState` (`GameplayStatics.GetGameState`)))
  (bind _output_get (set `self.CurrentOrder` (`/Game/Blueprints/BP_CarpenterGameState.CurrentOrder` _asbp_carpenter_game_state)))
  (if (`.IsActive_8_A735101046AA32811AC3FEAFDAA72CE0` (break `/Game/DataTypes/S_Order` _output_get))
    ; Product & Color Match  and Complete & Destroy
    (bind _returnvalue (`self.IsSameProductType` (`self.CurrentOrder`) (`self.CurrentProduct`)))
    (if _returnvalue
      (bind _returnvalue_2 (`self.IsSameColor` (`self.CurrentOrder`) (`self.CurrentProduct`)))
      (if _returnvalue_2
        (`KismetSystemLibrary.Delay` 0.5)
        (`self.ProcessDelivery` _currentorder_price_2)
        (else
          (`KismetSystemLibrary.Delay` 0.5)
          (`self.ProcessDelivery` (/ _currentorder_price 2))))
      (else
        (`KismetSystemLibrary.Delay` 0.5)
        (`self.ProcessDelivery` 0)))))

(fn `IsSameColor`
  (params (Order :type "/Game/DataTypes/S_Order Structure") (ProductType :type "/Game/Blueprints/Products/BP_Product Object Reference"))
  (returns (ReturnValue :type Boolean))
  ; Check Paint Color
  (return (`|EnumEquality` (`.PaintColor_5_79771EA043BC025B8733C5B69B837995` (break `/Game/DataTypes/S_Order` Order)) (`/Game/Blueprints/Products/BP_Product.Color` ProductType))))

(fn `IsSameProductType`
  (params (Order :type "/Game/DataTypes/S_Order Structure") (ProductType :type "/Game/Blueprints/Products/BP_Product Object Reference"))
  (returns (ReturnValue :type Boolean))
  ; Check Product Type
  (return (`|EnumEquality` (`.ProductType_4_D37A55584A89802943A0E1812A9D4E73` (break `/Game/DataTypes/S_Order` Order)) (`/Game/Blueprints/Products/BP_Product.ProductType` ProductType))))

(fn `ProcessDelivery`
  (params (Payment :type Integer))
  (bind _asbp_carpenter_game_mode (cast `/Game/Blueprints/BP_CarpenterGameMode` (`GameplayStatics.GetGameMode`)))
  (`/Game/Blueprints/BP_CarpenterGameMode.CompleteOrder` _asbp_carpenter_game_mode Payment)
  (`self.K2_DestroyActor` (`self.CurrentProduct`)))

(fn `UserConstructionScript`)