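; Order board actor that shows the carpenter game's current order on a widget.
; It binds to the game state's order-updated event and refreshes the widget, showing the active order or clearing the display.
; Separate functions spawn and destroy a half-scale preview product at a spawn point, copying the order's type and paint color, though nothing in this graph calls them.
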(event `self.ReceiveBeginPlay`
  (bind _asbp_carpenter_game_state (cast `/Game/Blueprints/BP_CarpenterGameState` (`GameplayStatics.GetGameState`)))
  (add `/Game/Blueprints/BP_CarpenterGameState.OnOrderUpdated` _asbp_carpenter_game_state (delegate `UpdateOrderDisplay`)))

(event `UpdateOrderDisplay`
  (`self.RefreshDisplay`))

(fn `DestroyPreview`
  ; Destroy Preview Object
  (`self.K2_DestroyActor` (`self.PreviewProduct`))
  (set `self.PreviewProduct` null))

(fn `RefreshDisplay`
  ; Refresh Order Display
  (bind _aswbp_order_interface (cast `/Game/Blueprints/UI/WBP_OrderInterface` (`WidgetComponent.GetWidget` (`self.Widget`))))
  (set `self.OrderInterface` _aswbp_order_interface)
  (bind _asbp_carpenter_game_state (cast `/Game/Blueprints/BP_CarpenterGameState` (`GameplayStatics.GetGameState`)))
  (bind (_currentorder_producttype _currentorder_paintcolor _currentorder_price _currentorder_isactive) (break `/Game/DataTypes/S_Order` (`/Game/Blueprints/BP_CarpenterGameState.CurrentOrder` _asbp_carpenter_game_state)))
  (if _currentorder_isactive
    (`/Game/Blueprints/UI/WBP_OrderInterface.UpdateDisplay` (`self.OrderInterface`) (`/Game/Blueprints/BP_CarpenterGameState.CurrentOrder` _asbp_carpenter_game_state))
    (else
      (`/Game/Blueprints/UI/WBP_OrderInterface.ClearDisplay` (`self.OrderInterface`)))))

(fn `SpawnPreview`
  (bind _previewspawnpoint (`self.PreviewSpawnPoint`))
  ; Spawn Preview Object
  (bind _returnvalue (`|SpawnActorFromClass` "/Game/Blueprints/Products/BP_Product.BP_Product_C" (`KismetMathLibrary.MakeTransform` (`SceneComponent.K2_GetComponentLocation` _previewspawnpoint) (`SceneComponent.K2_GetComponentRotation` _previewspawnpoint) (0.5 0.5 0.5)) "Undefined" "MultiplyWithRoot" null null))
  (bind _output_get (set `self.PreviewProduct` _returnvalue))
  (bind _asbp_carpenter_game_state (cast `/Game/Blueprints/BP_CarpenterGameState` (`GameplayStatics.GetGameState`)))
  (bind (_producttype _paintcolor) (break `/Game/DataTypes/S_Order` (`/Game/Blueprints/BP_CarpenterGameState.CurrentOrder` _asbp_carpenter_game_state)))
  (set `/Game/Blueprints/Products/BP_Product.ProductType` _producttype _output_get)
  (set `/Game/Blueprints/Products/BP_Product.Color` _paintcolor (`self.PreviewProduct`))
  (set `/Game/Blueprints/Products/BP_Product.IsPreview` true (`self.PreviewProduct`)))

(fn `UserConstructionScript`)