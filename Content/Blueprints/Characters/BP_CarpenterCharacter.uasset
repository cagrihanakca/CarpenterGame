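; BP_CarpenterCharacter is the networked player character that moves, looks, carries products, triggers paint buckets and clicks world widgets, with a budget HUD for the local player.
; Interact sphere-traces along the control rotation to pick up a product or trigger a paint bucket, or drops whatever is held.
; Server RPCs route carry, drop, paint and carving machine produce and selection requests.
; Carrying skips preview products and sets the product's CarryOwner before updating its carry state.
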(event `self.ReceiveBeginPlay`
  ; Input & HUD Setup
  (if (`self.IsLocallyControlled`)
    (`EnhancedInputSubsystemInterface.AddMappingContext` (subsystem `EnhancedInputLocalPlayerSubsystem`) "/Game/Input/IMC_Default.IMC_Default" 0 (struct))
    (bind _returnvalue (`|CreateWidget` "/Game/Blueprints/UI/WBP_BudgetHUD.WBP_BudgetHUD_C"))
    (`UserWidget.AddToViewport` _returnvalue 0)))

(event `EnhancedInput|/Game/Input/IA_Move`
  (params (ActionValue :type "Vector2D Structure") (ElapsedSeconds :type "Float (double-precision)") (TriggeredSeconds :type "Float (double-precision)") (InputAction :type "InputAction Object Reference" :default "/Game/Input/IA_Move.IA_Move"))
  (bind (_x _y) (`KismetMathLibrary.BreakVector2D` ActionValue))
  ; Player Movement
  (:`Triggered`
    (`self.AddMovementInput` (`KismetMathLibrary.GetForwardVector` (`self.GetControlRotation`)) _x)
    (`self.AddMovementInput` (`KismetMathLibrary.GetRightVector` (`self.GetControlRotation`)) _y)))

(event `EnhancedInput|/Game/Input/IA_Look`
  (params (ActionValue :type "Vector2D Structure") (ElapsedSeconds :type "Float (double-precision)") (TriggeredSeconds :type "Float (double-precision)") (InputAction :type "InputAction Object Reference" :default "/Game/Input/IA_Look.IA_Look"))
  (bind (_x _y) (`KismetMathLibrary.BreakVector2D` ActionValue))
  ; Camera Rotation
  (:`Triggered`
    (`self.AddControllerYawInput` _x)
    (`self.AddControllerPitchInput` (* -1.0 _y))))

(event `EnhancedInput|/Game/Input/IA_Interact`
  (params (ActionValue :type Boolean) (ElapsedSeconds :type "Float (double-precision)") (TriggeredSeconds :type "Float (double-precision)") (InputAction :type "InputAction Object Reference" :default "/Game/Input/IA_Interact.IA_Interact"))
  ; Interact System
  (:`Started`
    (if (`self.IsCarrying`)
      (`self.ServerDropProduct`)
      (else
        (bind _hit_actor (`self.Interact`))
        (bind _asbp_product (cast `/Game/Blueprints/Products/BP_Product` _hit_actor)
          (:`then`
            (`self.ServerCarryProduct` _asbp_product))
          (:`CastFailed`
            (bind _asbp_paint_bucket (cast `/Game/Blueprints/Machines/BP_PaintBucket` _hit_actor))
            (`self.ServerTriggerPaint` _asbp_paint_bucket)))))))

(event `Key|LeftMouseButton`
  (params (Key :type "Key Structure"))
  (bind _widgetinteraction (`self.WidgetInteraction`))
  ; Widget Interaction - Click
  (:`Pressed`
    (`WidgetInteractionComponent.PressPointerKey` _widgetinteraction "LeftMouseButton"))
  (:`Released`
    (`WidgetInteractionComponent.ReleasePointerKey` _widgetinteraction "LeftMouseButton")))

(event `ServerDropProduct`
  ; Server RPC - Drop
  (`self.DropProduct`))

(event `ServerCarryProduct`
  (params (Product :type "/Game/Blueprints/Products/BP_Product Object Reference"))
  ; Server RPC - Carry
  (`self.CarryProduct` Product))

(event `ServerRequestProduce`
  (params (CarvingMachine :type "/Game/Blueprints/Machines/BP_CarvingMachine Object Reference") (`Product Type` :type "/Game/DataTypes/E_ProductType Enum" :default "NewEnumerator0"))
  ; Server RPC - Request Produce
  (`/Game/Blueprints/Machines/BP_CarvingMachine.ProduceObject` CarvingMachine `Product Type`))

(event `ServerRequestSelect`
  (params (CarvingMachine :type "/Game/Blueprints/Machines/BP_CarvingMachine Object Reference") (ProductType :type "/Game/DataTypes/E_ProductType Enum" :default "NewEnumerator0"))
  ; Server RPC - Request Select
  (`/Game/Blueprints/Machines/BP_CarvingMachine.SetSelection` CarvingMachine ProductType))

(event `ServerTriggerPaint`
  (params (PaintBucket :type "/Game/Blueprints/Machines/BP_PaintBucket Object Reference"))
  ; Server RPC - Trigger Paint
  (`/Game/Blueprints/Machines/BP_PaintBucket.TriggerPaint` PaintBucket))

(fn `CarryProduct`
  (params (Product :type "/Game/Blueprints/Products/BP_Product Object Reference"))
  ; Carry Product
  (if (not (`/Game/Blueprints/Products/BP_Product.IsPreview` Product))
    (bind _output_get (set `self.HeldProduct` Product))
    (set `/Game/Blueprints/Products/BP_Product.CarryOwner` self _output_get)
    (`/Game/Blueprints/Products/BP_Product.HandleCarryState` (`self.HeldProduct`))
    (set `self.IsCarrying` true)))

(fn `DropProduct`
  ; Drop Product
  (set `/Game/Blueprints/Products/BP_Product.CarryOwner` null (`self.HeldProduct`))
  (`/Game/Blueprints/Products/BP_Product.HandleCarryState` (`self.HeldProduct`))
  (set `self.HeldProduct` null)
  (set `self.IsCarrying` false))

(fn `Interact`
  (returns (`Hit Actor` :type "Actor Object Reference"))
  (bind _returnvalue (+ (`self.K2_GetActorLocation`) (0.0 0.0 75.0)))
  ; Interact - Line Trace
  (bind _outhit (`KismetSystemLibrary.SphereTraceSingle` _returnvalue (+ _returnvalue (* (`KismetMathLibrary.GetForwardVector` (`self.GetControlRotation`)) 400.0)) 30.0 "TraceTypeQuery1"))
  (return (`.HitActor` (`GameplayStatics.BreakHitResult` _outhit))))

(fn `UserConstructionScript`)