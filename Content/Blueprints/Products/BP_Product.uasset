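; BP_Product is a carryable product actor with a shape type and a paint color.
; ProductType, Color and CarryOwner use RepNotify, so each OnRep refreshes the mesh, material or carry state.
; A valid CarryOwner turns off physics, attaches the product to that owner's HoldPoint and makes its mesh ignore the Camera channel.
; Without a valid owner, the product detaches in world space, simulates physics and blocks the Camera channel again.
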(fn `HandleCarryState`
  ; Attach & Detach and Physics Toggle
  (`/Engine/EditorBlueprintResources/StandardMacros.IsValid` (`self.CarryOwner`)
    (:`Is Valid`
      (`PrimitiveComponent.SetSimulatePhysics` (`self.StaticMesh`) false)
      (`self.K2_AttachToComponent` (`/Game/Blueprints/Characters/BP_CarpenterCharacter.HoldPoint` (`self.CarryOwner`)) "None" "SnapToTarget" "KeepRelative" "KeepRelative")
      (`PrimitiveComponent.SetCollisionResponseToChannel` (`self.StaticMesh`) "ECC_Camera" "ECR_Ignore"))
    (:`Is Not Valid`
      (`self.K2_DetachFromActor` "KeepWorld" "KeepWorld")
      (`PrimitiveComponent.SetSimulatePhysics` (`self.StaticMesh`) true)
      (`PrimitiveComponent.SetCollisionResponseToChannel` (`self.StaticMesh`) "ECC_Camera" "ECR_Block"))))

(fn `OnRep_CarryOwner`
  ; OnRep - Handle Carry State
  (`self.HandleCarryState`))

(fn `OnRep_Color`
  ; OnRep - Set Paint Material
  (`self.SetPaintMaterial`))

(fn `OnRep_ProductType`
  ; OnRep - Set Product Mesh
  (`self.SetProductMesh`))

(fn `SetPaintMaterial`
  (bind _staticmesh (`self.StaticMesh`))
  ; Set Material by Paint Color
  (switch `/Game/DataTypes/E_PaintColor` (`self.Color`)
    (:`NewEnumerator0`
      (`PrimitiveComponent.SetMaterial` _staticmesh 0 "/Game/Materials/M_Red.M_Red"))
    (:`NewEnumerator1`
      (`PrimitiveComponent.SetMaterial` _staticmesh 0 "/Game/Materials/M_Green.M_Green"))
    (:`NewEnumerator2`
      (`PrimitiveComponent.SetMaterial` _staticmesh 0 "/Game/Materials/M_Blue.M_Blue"))
    (:`NewEnumerator3`
      (`PrimitiveComponent.SetMaterial` _staticmesh 0 "/Game/Materials/M_Yellow.M_Yellow"))))

(fn `SetProductMesh`
  (bind _staticmesh (`self.StaticMesh`))
  ; Set Mesh by Product Type
  (switch `/Game/DataTypes/E_ProductType` (`self.ProductType`)
    (:`NewEnumerator0`
      (`StaticMeshComponent.SetStaticMesh` _staticmesh "/Engine/BasicShapes/Cube.Cube"))
    (:`NewEnumerator1`
      (`StaticMeshComponent.SetStaticMesh` _staticmesh "/Engine/BasicShapes/Cylinder.Cylinder"))
    (:`NewEnumerator2`
      (`StaticMeshComponent.SetStaticMesh` _staticmesh "/Engine/BasicShapes/Sphere.Sphere"))
    (:`NewEnumerator3`
      (`StaticMeshComponent.SetStaticMesh` _staticmesh "/Engine/BasicShapes/Cone.Cone"))))

(fn `UserConstructionScript`)